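; Player character with flipbook sprite for side-on platforming: X-axis movement, jump, wall jump and velocity-based dash.
; Airborne jumps trace along the forward axis past the capsule, launching away from walls or falling back to a jump capped by JumpCount, which landing resets.
; Jump and landing spawn dust and drive timelines that squash and stretch actor scale.
; Left/right flipbook switching is disconnected; the construction script sets jump tuning.
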(event Custom|wall%20Jump
  (bind _returnvalue (Transformation|GetActorForwardVector))
  ;[1 1 1] Wall Jump
  (bind (_outhit _returnvalue_2) (Collision|LineTraceByChannel (- (Transformation|GetActorLocation) (* _returnvalue (+ (Components|Capsule|GetScaledCapsuleRadius (Variables|Collision|GetCapsuleComponent)) 15.0))) (+ (Transformation|GetActorLocation) (* _returnvalue (+ (Components|Capsule|GetScaledCapsuleRadius (Variables|Collision|GetCapsuleComponent)) 15.0))) "TraceTypeQuery1" true 0 "None"))
  (if _returnvalue_2
    (Character|LaunchCharacter (Math|Vector|MakeVector (* (Math|Float|Sign(Float) (- (.x (Transformation|GetActorLocation)) (.x (.Location (Collision|BreakHitResult _outhit))))) 4.5e+02) 0.0 (Variables|/Script/Engine.CharacterMovementComponent|GetJumpZVelocity (Variables|Character|GetCharacterMovement))) false false)
    (elif (< (Variables|Default|GetjumpCount) 2)
      (Character|Jump)
      (Variables|Default|SetjumpCount (+ (Variables|Default|GetjumpCount) 1)))))

(event Custom|jumpFX
  ;[1 1 1] jump animatio
  (Effects|SpawnEmitteratLocation "/Game/NewFolder/Art/particles/pDust.pDust" (Transformation|GetWorldLocation (Variables|Default|Getdust%20box)))
  (bind _squash (Timeline|Timeline_0 PlayFromStart)
    (:Update
      (Transformation|SetActorRelativeScale3D (Math|Vector|Lerp(Vector) "1.000000,1.000000,1.000000" "0.250000,1.000000,2.000000" _squash)))))

(event Custom|LandingFx
  ;[1 1 1] Landed animation
  (Effects|SpawnEmitteratLocation "/Game/NewFolder/Art/particles/pDust.pDust" (Transformation|GetWorldLocation (Variables|Default|Getdust%20box)))
  (Sprite|SetFlipbook (Variables|Default|GetSprite) "/Game/NewFolder/Art/flipBook/IdleSQare.IdleSQare")
  (bind _squash (Timeline|Timeline_1 Play)
    (:Update
      (Transformation|SetActorRelativeScale3D (Math|Vector|Lerp(Vector) "1.000000,1.000000,1.000000" "2.000000,1.000000,0.250000" _squash)))))

(event EventOnLanded
  (params (Hit :type Hit%20Result%20Structure%20%28by%20ref%29))
  ;[1 1 1] Landed(Reset jump Count)
  (Variables|Default|SetjumpCount 0)
  (CallFunction|LandingFx))

(event Input|ActionEvents|InputActionJump
  (params (Key :type Key%20Structure))
  ;[1 1 1] Jumping
  (:Pressed
    (if (AI|Components|NavMovement|IsFalling (Variables|Character|GetCharacterMovement))
      (CallFunction|WallJump)
      (CallFunction|JumpFX)
      (else
        (Character|Jump)
        (Sprite|SetFlipbook (Variables|Default|GetSprite) "/Game/NewFolder/Art/flipBook/JumpSQare.JumpSQare")
        (Variables|Default|SetjumpCount (+ (Variables|Default|GetjumpCount) 1))
        (CallFunction|JumpFX)
        (CallFunction|JumpFX))))
  (:Released
    (Character|StopJumping)))

(event Input|ActionEvents|InputActionDash
  (params (Key :type Key%20Structure))
  (bind _returnvalue (Transformation|GetVelocity))
  ;[1 1 1] Dash
  (:Pressed
    (if (Math|Vector|NotEqual(Vector) _returnvalue "0, 0, 0" 0.0001)
      (if (AI|Components|NavMovement|IsFalling (Variables|Character|GetCharacterMovement))
        (Character|LaunchCharacter (* (+ _returnvalue "0, 0, 0") "1.500000,1.500000,1.500000") false false)
        (else
          (Character|LaunchCharacter (* (+ _returnvalue "0, 0,1.000000") "1.500000,1.500000,250.000000") false false))))))

(event Input|AxisEvents|InputAxisRight
  (params (AxisValue :type Float%20%28single-precision%29))
  ;[1 1 1] Movement control
  (Pawn|Input|AddMovementInput "1.000000, 0, 0" AxisValue false))

(fn ConstructionScript
  (Variables|/Script/Engine.CharacterMovementComponent|SetJumpZVelocity (Variables|Character|GetCharacterMovement) 4e+02)
  (Variables|Default|SetJumpMaxHoldTime 0.2)
  (Variables|Default|SetjumpCount 0))